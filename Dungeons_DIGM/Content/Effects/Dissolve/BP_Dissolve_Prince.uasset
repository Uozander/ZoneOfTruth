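; BP_Dissolve_Prince plays a timed dissolve effect on a static mesh, paired with Niagara particles.
; On BeginPlay it creates a dynamic material instance, sets its Fade parameter fully up, then waits briefly before starting a timeline.
; The timeline drives the particle spawn rate and amount down to zero while remapping the same blend to sweep Fade from 1 to -1, keeping particles and material in step.
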(event EventBeginPlay
  (bind _returnvalue (Rendering|Material|CreateDynamicMaterialInstance (Variables|Default|GetStaticMesh) 0 "/Game/Characters/Prince/Merged_Extract1.Merged_Extract1" "None" :!class /Script/Engine.PrimitiveComponent))
  (bind _output_get (Variables|Default|SetFade _returnvalue))
  (Rendering|Material|SetScalarParameterValue _output_get "Fade" 1.0 :!class /Script/Engine.MaterialInstanceDynamic)
  (Utilities|FlowControl|Delay 2.0)
  (bind _newtrack_0 (Timeline|Timeline_0 PlayFromStart)
    (:Update
      (Niagara|SetNiagaraVariable(Float) (Variables|Default|GetNiagara) "Spawn Rate" (Math|Float|Lerp 5e+04 0.0 _newtrack_0))
      (Niagara|SetNiagaraVariable(Float) (Variables|Default|GetNiagara) "Amount" (Math|Float|Lerp 1.0 0.0 _newtrack_0))
      (Rendering|Material|SetScalarParameterValue (Variables|Default|GetFade) "Fade" (- (* (Math|Float|Lerp 1.0 0.0 _newtrack_0) 2.0) 1.0) :!class /Script/Engine.MaterialInstanceDynamic))))

(fn ConstructionScript)