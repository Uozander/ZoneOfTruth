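; Dissolve effect Blueprint for the Kelrax character that runs automatically on BeginPlay.
; It creates dynamic material instances for the body and head meshes, then starts a separate timeline for each after a short delay.
; Each timeline sweeps the material's Fade parameter while lowering its Niagara system's spawn rate and raising its Amount, keeping particles in step with the dissolve.
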(event EventBeginPlay
  (Utilities|FlowControl|Sequence
    (:then_0
      (bind _returnvalue (Rendering|Material|CreateDynamicMaterialInstance (Variables|Default|GetKelrax_Bod_Merged_Extract5) 0 "/Game/Characters/Kelrax/M_Kelrax_Bod.M_Kelrax_Bod" "None" :!class /Script/Engine.PrimitiveComponent))
      (Variables|Default|SetFadeBody _returnvalue)
      (Utilities|FlowControl|Delay 1.0)
      (bind _newtrack_0 (Timeline|Timeline PlayFromStart)
        (:Update
          (Niagara|SetNiagaraVariable(Float) (Variables|Default|GetNiagara) "Spawn Rate" (Math|Float|Lerp 5e+04 0.0 _newtrack_0))
          (Niagara|SetNiagaraVariable(Float) (Variables|Default|GetNiagara) "Amount" (Math|Float|Lerp 0.0 0.5 _newtrack_0))
          (Rendering|Material|SetScalarParameterValue (Variables|Default|GetFadeBody) "Fade" (- (* (Math|Float|Lerp 0.0 1.0 _newtrack_0) 2.0) 1.0) :!class /Script/Engine.MaterialInstanceDynamic))))
    (:then_1
      (bind _returnvalue_2 (Rendering|Material|CreateDynamicMaterialInstance (Variables|Default|GetKelrax_Bod_Merged_Extract6) 0 "/Game/Characters/Kelrax/M_Kelrax.M_Kelrax" "None" :!class /Script/Engine.PrimitiveComponent))
      (Variables|Default|SetFadeHead _returnvalue_2)
      (Utilities|FlowControl|Delay 1.0)
      (bind _newtrack_0_2 (Timeline|Timeline_1 PlayFromStart)
        (:Update
          (Niagara|SetNiagaraVariable(Float) (Variables|Default|GetNiagara1) "Spawn Rate" (Math|Float|Lerp 5e+04 0.0 _newtrack_0_2))
          (Niagara|SetNiagaraVariable(Float) (Variables|Default|GetNiagara1) "Amount" (Math|Float|Lerp 0.0 0.5 _newtrack_0_2))
          (Rendering|Material|SetScalarParameterValue (Variables|Default|GetFadeHead) "Fade" (- (* (Math|Float|Lerp 0.0 1.0 _newtrack_0_2) 2.0) 1.0) :!class /Script/Engine.MaterialInstanceDynamic))))))

(fn ConstructionScript)