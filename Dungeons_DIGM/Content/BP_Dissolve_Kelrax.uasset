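; BP_Dissolve_Kelrax is an actor that dissolves a skeletal mesh with Niagara particles shortly after play begins.
; BeginPlay creates a dynamic MAT_KP material on the mesh, waits briefly, then plays a timeline.
; The timeline ramps the material's Fade parameter from -1 to 1 while driving the Niagara Amount up and Spawn Rate down.
; A second timeline holds the reverse transition but is never triggered.
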(event EventBeginPlay
  (bind _returnvalue (Rendering|Material|CreateDynamicMaterialInstance (Variables|Default|GetSkeletalMesh) 0 "/Game/MAT_KP.MAT_KP" "None" :!class /Script/Engine.PrimitiveComponent))
  (Variables|Default|SetFade _returnvalue)
  (Utilities|FlowControl|Delay 2.0)
  (bind _newtrack_0 (Timeline|Timeline PlayFromStart)
    (:Update
      (Niagara|SetNiagaraVariable(Float) (Variables|Default|GetNiagara) "Spawn Rate" (Math|Float|Lerp 5e+04 0.0 _newtrack_0))
      (Niagara|SetNiagaraVariable(Float) (Variables|Default|GetNiagara) "Amount" (Math|Float|Lerp 0.0 1.0 _newtrack_0))
      (Rendering|Material|SetScalarParameterValue (Variables|Default|GetFade) "Fade" (- (* (Math|Float|Lerp 0.0 1.0 _newtrack_0) 2.0) 1.0) :!class /Script/Engine.MaterialInstanceDynamic))))

(fn ConstructionScript)